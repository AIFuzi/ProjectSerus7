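; BP_DamageTestrLow is a test character that takes damage and ragdolls when its health runs out.
; AnyDamage passes the negated damage to its health component, whose HealthEnd event calls Dead.
; Dead disables movement, turns on mesh physics simulation and leaves the capsule with physics-only collision.
; A delayed call to Dead is left unconnected and never runs.
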(event HealthEnd(BP_HealthComponent)
  (CallFunction|Dead))

(event Game|Damage|EventAnyDamage
  (params (Damage :type Float%20%28single-precision%29) (DamageType :type Damage%20Type%20Object%20Reference) (InstigatedBy :type Controller%20Object%20Reference) (DamageCauser :type Actor%20Object%20Reference))
  (Default|ChangeHealth (Variables|Default|GetBP_HealthComponent) (* Damage -1.0)))

(event EventBeginPlay)

(fn ConstructionScript)

(fn Dead
  (bind _mesh (Variables|Character|GetMesh))
  (Pawn|Components|CharacterMovement|DisableMovement (Variables|Character|GetCharacterMovement))
  (Collision|SetCollisionEnabled _mesh "QueryAndPhysics")
  (Physics|SetSimulatePhysics _mesh true)
  (Collision|SetCollisionEnabled (Variables|Collision|GetCapsuleComponent) "PhysicsOnly"))