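; BP_DamageTestrMedium is a character in the Test folder that, judging by its name, serves as a damage test target and ragdolls when its health runs out.
; The HealthEnd event of BP_HealthComponent calls Dead, which disables movement, enables mesh collision and physics simulation, and leaves the capsule on physics-only collision.
; BeginPlay is empty, and a delayed call to Dead is left unconnected.
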(event HealthEnd(BP_HealthComponent)
  (CallFunction|Dead))

(event EventBeginPlay)

(fn ConstructionScript)

(fn Dead
  (bind _mesh (Variables|Character|GetMesh))
  (Pawn|Components|CharacterMovement|DisableMovement (Variables|Character|GetCharacterMovement))
  (Collision|SetCollisionEnabled _mesh "QueryAndPhysics")
  (Physics|SetSimulatePhysics _mesh true)
  (Collision|SetCollisionEnabled (Variables|Collision|GetCapsuleComponent) "PhysicsOnly"))