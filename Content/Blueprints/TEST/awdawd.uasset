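; Test actor that acts as a rotating damage beam, cast from a Cube component.
; Each tick it line-traces forward from the cube against static, dynamic and pawn objects, drawing the debug line, and applies damage to any actor hit.
; It then adds a fixed local rotation to the cube, so rotation speed and damage rate both depend on frame rate.
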(event EventTick
  (params (DeltaSeconds :type Float%20%28single-precision%29))
  (bind _cube (Variables|Default|GetCube))
  (bind _returnvalue (Transformation|GetWorldLocation _cube))
  (Utilities|FlowControl|Sequence
    (:then_0
      (bind (_outhit _returnvalue_2) (Collision|LineTraceForObjects _returnvalue (+ _returnvalue (* (Math|Vector|GetForwardVector _cube) 1e+03)) (Utilities|Array|MakeArray "ObjectTypeQuery1" "ObjectTypeQuery2" "ObjectTypeQuery3") false (Utilities|Array|MakeArray self) "ForDuration" true "(R=1.000000,G=0.000000,B=0.000000,A=1.000000)" "(R=0.000000,G=1.000000,B=0.000000,A=1.000000)" 0.0))
      (if _returnvalue_2
        (Game|Damage|ApplyDamage (.HitActor (Collision|BreakHitResult _outhit)) 3.0 (Game|GetInstigatorController) self)))
    (:then_1
      (Transformation|AddLocalRotation (Variables|Default|GetCube) "0,3.000000, 0" false false))))

(fn ConstructionScript)